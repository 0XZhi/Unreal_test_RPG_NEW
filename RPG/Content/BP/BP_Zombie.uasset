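; Zombie enemy Blueprint that wanders to random reachable points, chases the player woman when seen, and attacks her.
; PawnSensing drives AIMoveTo toward BP_Woman, then a DoOnce-gated attack montage resets and resumes wandering; the hurt event also triggers both.
; The attack collision damages her on overlap, with a function toggling its overlap events.
; The damage function lowers health and plays hit or dying montages; Tick destroys the zombie after a delay.
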(event `self.ReceiveBeginPlay`
  ;[1 1 1] 隨機走動
  (if (not (`self.是否死亡`))
    (`/Engine/EditorBlueprintResources/StandardMacros.IsValid` (`self.玩家物件`)
      (:`Is Not Valid`
        (`|AIMoveTo` self (`NavigationSystemV1.K2_GetRandomReachablePointInRadius` (`SceneComponent.K2_GetComponentLocation` (`self.Mesh`)) (`KismetMathLibrary.RandomFloatInRange` 500.0 1000.0) null null) null :!label _label
          (:`OnSuccess`
            _)
          (:`OnFail`
            _))
        (`KismetSystemLibrary.Delay` (`KismetMathLibrary.RandomFloatInRange` 1.0 2.0))
        (if (not (`self.攻擊玩家`))
          (goto _label))))))

(event `受傷事件_Event`
  (set `self.攻擊玩家` false)
  (`|ExecutionSequence`
    (:`then_0`
      (goto _label))
    (:`then_1`
      ;[1 1 1] 攻擊事件
      (`/Engine/EditorBlueprintResources/StandardMacros.DoOnce` false :!label _label_2
        (:`Completed`
          (`|PlayMontage` (`self.Mesh`) "/Game/Animation/ZombieAni/Zombie_Attack_Montage.Zombie_Attack_Montage" 1.5
            (:`then`
              (set `self.攻擊玩家` true)
              (set `self.玩家物件` null))
            (:`OnCompleted`
              (set `self.攻擊玩家` false)
              (`KismetSystemLibrary.Delay` 0.2)
              (`|ExecutionSequence`
                (:`then_0`
                  (goto _label_2 :!via `Reset`))
                (:`then_1`
                  (goto _label))))))))))

(event `self.PawnSensing.OnSeePawn`
  (params (Pawn :type "Pawn Object Reference"))
  ;[1 1 1] 攻擊事件
  (if (not (`self.攻擊玩家`))
    (bind _asbp_woman (cast `/Game/BP/BP_Woman` Pawn))
    (bind _output_get (set `self.玩家物件` _asbp_woman))
    (`|AIMoveTo` self (0.0 0.0 0.0) _output_get
      (:`OnSuccess`
        (goto _label_2)))))

(event `self.ReceiveTick`
  (params (DeltaSeconds :type "Float (single-precision)"))
  (if (<= (`self.僵屍血量`) 0.0)
    (set `self.是否死亡` true)
    (`KismetSystemLibrary.Delay` 3.0)
    (`self.K2_DestroyActor` self)))

(event `self.攻擊碰撞區域.OnComponentBeginOverlap`
  (params (OverlappedComponent :type "PrimitiveComponent Object Reference") (OtherActor :type "Actor Object Reference") (OtherComp :type "PrimitiveComponent Object Reference") (OtherBodyIndex :type Integer) (bFromSweep :type Boolean) (SweepResult :type "HitResult Structure (by ref)"))
  (bind _asbp_woman (cast `/Game/BP/BP_Woman` OtherActor))
  (`/Game/BP/BP_Woman.玩家受傷` _asbp_woman 0.3))

(fn `UserConstructionScript`)

(fn `受傷`
  (params (`被扣血量` :type "Float (double-precision)"))
  (if (not (`self.是否死亡`))
    (set `self.僵屍血量` (- (`self.僵屍血量`) `被扣血量`))
    (`self.PlayAnimMontage` self "/Game/Animation/ZombieAni/Zombie_Hit_Montage.Zombie_Hit_Montage" 1.0 "None")
    (if (<= (`self.僵屍血量`) 0.0)
      (`self.PlayAnimMontage` self "/Game/Animation/ZombieAni/Zombie_Dying_Montage.Zombie_Dying_Montage" 1.0 "None"))))

(fn `怪物是否顯示攻擊碰撞`
  (params (`攻擊顯示` :type Boolean :default false))
  (set `PrimitiveComponent.bGenerateOverlapEvents` `攻擊顯示` (`self.攻擊碰撞區域`)))